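; Gameplay ability that lets a character find and trigger interactions with nearby objects.
; On activation, a short-range line trace task, with debug drawing on, scans from the owning actor and updates the available interaction options when detected interactables change.
; In parallel, an input-press wait task triggers the current interaction, prints a debug string, and re-arms itself after each press.
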(event Custom|Look%20for%20Interactables
  (bind _interactableoptions (|WaitforInteractableTargetsLineTrace (Utilities|Struct|MakeInteractionQuery (Ability|GetAvatarActorfromActorInfo) (.AsController (Utilities|Casting|CastToController (Ability|GetOwningActorfromActorInfo)))) "(Name=\"NoCollision\")" (Class|GameplayAbility|MakeTargetLocationInfofromOwnerActor) 2e+02 0.1 true)
    (:InteractableObjectsChanged
      (Class|ControlGameplayAbilityInteract|UpdateInteractions _interactableoptions))))

(event Custom|InteractPressScan
  (Ability|Tasks|WaitInputPress false
    (:OnPress
      (Development|PrintString "Interact")
      (Utilities|FlowControl|Sequence
        (:then_0
          (Class|ControlGameplayAbilityInteract|TriggerInteraction))
        (:then_1
          (CallFunction|InteractPressScan))))))

(event Ability|EventActivateAbility
  (CallFunction|LookforInteractables)
  (CallFunction|InteractPressScan))

(event Ability|EventOnEndAbility
  (params (bWasCancelled :type Boolean)))