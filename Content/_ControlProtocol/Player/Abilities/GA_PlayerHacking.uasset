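; Player hacking gameplay ability that finds hackable objects and triggers hacks on input.
; On activation, a line-trace task scans from the owning actor with a hacking query, debug drawing on, and passes changed options to UpdateHackings.
; In parallel, an input-press wait prints a debug string, calls TriggerHacking, then re-arms itself for repeated presses.
; The graph never ends the ability.
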(event Custom|Look%20For%20Hackables
  (bind _hackableoptions (|WaitforHackableTargetsSingleLineTrace (Utilities|Struct|MakeHackingQuery (Ability|GetAvatarActorfromActorInfo) (.AsController (Utilities|Casting|CastToController (Ability|GetOwningActorfromActorInfo)))) "(Name=\"NoCollision\")" (Class|GameplayAbility|MakeTargetLocationInfofromOwnerActor) 8e+02 0.1 true)
    (:HackableObjectsChanged
      (Class|ControlGameplayAbilityHack|UpdateHackings _hackableoptions))))

(event Custom|HackPressSacn
  (Ability|Tasks|WaitInputPress false
    (:OnPress
      (Development|PrintString "Hack")
      (Utilities|FlowControl|Sequence
        (:then_0
          (Class|ControlGameplayAbilityHack|TriggerHacking))
        (:then_1
          (CallFunction|HackPressSacn))))))

(event Ability|EventActivateAbility
  ;[0.15 0.15 0.15 0.5] Comment
  ;;[0.15 0.15 0.15 0.5] Comment
  (CallFunction|LookforHackables)
  (CallFunction|HackPressSacn))

(event Ability|EventOnEndAbility
  (params (bWasCancelled :type Boolean)))